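; BP_Switch is a toggle switch device that acts as a power source with an output port and no inputs.
; The construction script sets its on state from StartOn, and BeginPlay constructs the ports.
; Player interaction flips the state and returns the switch itself.
; IsOutputPowered reports that state for an output port that passes the IsPortOwned check.
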(event `self.ReceiveBeginPlay`
  (`self.ConstructPorts` 0 true))

(fn `IsOutputPowered`
  (params (Index :type Integer))
  (returns (IsPowered :type Boolean))
  (if (`self.IsPortOwned` (`|GetArrayItem` (`self.Outputs`) Index))
    (return (`self.IsOn`))))

(fn `OnInteract`
  (params (Player :type "/Game/Blueprints/BP_PlayerCharacter Object Reference"))
  (returns (Interactable :type "Actor Object Reference"))
  (`|ExecutionSequence`
    (:`then_0`
      (set `self.IsOn` (not (`self.IsOn`))))
    (:`then_1`
      (return self))))

(fn `UserConstructionScript`
  (`parent.UserConstructionScript`)
  (set `self.IsOn` (`self.StartOn`)))