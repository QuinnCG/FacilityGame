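; BP_Device is a device with power input and output ports, apparently a base for powered devices.
; ConstructPorts creates a given number of BP_PowerInput objects and an optional BP_PowerOutput, each referencing the owning device.
; Connect links ports by setting the destination's Source, while IsPortOwned checks whether a port belongs to the device.
; IsOutputPowered always returns false here, and GetOutput returns the first output.
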(fn `Connect`
  (params (Source :type "/Game/Blueprints/BP_PowerOutput Object Reference") (Destination :type "/Game/Blueprints/BP_PowerInput Object Reference"))
  (set `/Game/Blueprints/BP_PowerInput.Source` Source Destination))

(fn `ConstructPorts`
  (params (InputCount :type Integer) (HasOutput :type Boolean))
  (`|ExecutionSequence`
    (:`then_0`
      (for _ (range 1 (+ (`local.InputCount`) 1))
        (bind _returnvalue (`|GenericCreateObject` self "/Game/Blueprints/BP_PowerInput.BP_PowerInput_C" self))
        (`KismetArrayLibrary.Array_Add` (`self.Inputs`) _returnvalue)))
    (:`then_1`
      (if HasOutput
        (bind _returnvalue_2 (`|GenericCreateObject` self "/Game/Blueprints/BP_PowerOutput.BP_PowerOutput_C" self))
        (`KismetArrayLibrary.Array_Add` (`self.Outputs`) _returnvalue_2)))))

(fn `GetOutput`
  (returns (Output :type "/Game/Blueprints/BP_PowerOutput Object Reference"))
  (return (`|GetArrayItem` (`self.Outputs`))))

(fn `IsOutputPowered`
  (params (Index :type Integer))
  (returns (IsPowered :type Boolean))
  (return false))

(fn `IsPortOwned`
  (params (Port :type "/Game/Blueprints/BP_PowerPort Object Reference"))
  (returns (IsOwned :type Boolean))
  (bind _asbp_power_input (cast `/Game/Blueprints/BP_PowerInput` Port)
    (:`then`
      (if (not (`KismetArrayLibrary.Array_Contains` (`self.Inputs`) _asbp_power_input))
        (bind _asbp_power_output (cast `/Game/Blueprints/BP_PowerOutput` Port :!label _label)
          (:`then`
            (if (`KismetArrayLibrary.Array_Contains` (`self.Outputs`) _asbp_power_output)
              _
              (else
                (return false))))
          (:`CastFailed`
            (return false)))))
    (:`CastFailed`
      (goto _label)))
  (return true))

(fn `UserConstructionScript`)