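; BP_Logger is a device with one input port and no output that prints a message to the screen when powered.
; Each tick it polls whether its Source output is powered and, if so, prints Message in its Color.
; A Gate closes after the print and reopens once power drops, so the polling acts as a rising-edge trigger that prints once per power-up.
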(event `self.ReceiveBeginPlay`
  (`self.ConstructPorts` 1))

(event `self.ReceiveTick`
  (params (DeltaSeconds :type "Float (single-precision)"))
  (if (`/Game/Blueprints/BP_PowerPort.IsPowered` (`self.GetOutput` (`self.Source`)))
    (`|ExecutionSequence`
      (:`then_0`
        (`/Engine/EditorBlueprintResources/StandardMacros.Gate` false :!label _label
          (:`Exit`
            (`KismetSystemLibrary.PrintString` (`self.Message`) true true (`self.Color`)))))
      (:`then_1`
        (goto _label :!via `Close`)))
    (else
      (goto _label :!via `Open`))))

(fn `UserConstructionScript`
  (`parent.UserConstructionScript`))