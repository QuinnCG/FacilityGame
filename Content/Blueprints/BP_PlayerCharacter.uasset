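; Player character Blueprint that handles movement, looking, jumping, crouching and interaction through Enhanced Input, and creates the HUD on BeginPlay.
; The construction script derives walk and crouch speeds from MoveSpeed, and LookSensitivity scales look input.
; Interact line-traces from the camera up to InteractReach and calls OnInteract on actors implementing BPI_Interactable.
; Engine AnyDamage events are forwarded to BPHealthComponent unless player controller 0 instigated them.
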(event `EnhancedInput|/Game/Input/IA_MoveForward`
  (params (ActionValue :type "Float (double-precision)") (ElapsedSeconds :type "Float (double-precision)") (TriggeredSeconds :type "Float (double-precision)") (InputAction :type "InputAction Object Reference" :default "/Game/Input/IA_MoveForward.IA_MoveForward"))
  (:`Triggered`
    (`self.AddMovementInput` (`self.GetActorForwardVector`) ActionValue)))

(event `EnhancedInput|/Game/Input/IA_MoveRight`
  (params (ActionValue :type "Float (double-precision)") (ElapsedSeconds :type "Float (double-precision)") (TriggeredSeconds :type "Float (double-precision)") (InputAction :type "InputAction Object Reference" :default "/Game/Input/IA_MoveRight.IA_MoveRight"))
  (:`Triggered`
    (`self.AddMovementInput` (`self.GetActorRightVector`) ActionValue)))

(event `EnhancedInput|/Game/Input/IA_LookUp`
  (params (ActionValue :type "Float (double-precision)") (ElapsedSeconds :type "Float (double-precision)") (TriggeredSeconds :type "Float (double-precision)") (InputAction :type "InputAction Object Reference" :default "/Game/Input/IA_LookUp.IA_LookUp"))
  (:`Triggered`
    (`self.AddControllerPitchInput` (* ActionValue (`self.LookSensitivity`))) ; Pitch is rotating on the horizontal-axis
  ))

(event `EnhancedInput|/Game/Input/IA_LookRight`
  (params (ActionValue :type "Float (double-precision)") (ElapsedSeconds :type "Float (double-precision)") (TriggeredSeconds :type "Float (double-precision)") (InputAction :type "InputAction Object Reference" :default "/Game/Input/IA_LookRight.IA_LookRight"))
  (:`Triggered`
    (`self.AddControllerYawInput` (* (`self.LookSensitivity`) ActionValue)) ; Pitch is rotating on the vertical-axis
  ))

(event `EnhancedInput|/Game/Input/IA_Jump`
  (params (ActionValue :type Boolean) (ElapsedSeconds :type "Float (double-precision)") (TriggeredSeconds :type "Float (double-precision)") (InputAction :type "InputAction Object Reference" :default "/Game/Input/IA_Jump.IA_Jump"))
  (:`Started`
    (`self.Jump`))
  (:`Canceled`
    (`self.StopJumping`)))

(event `EnhancedInput|/Game/Input/IA_Crouch`
  (params (ActionValue :type Boolean) (ElapsedSeconds :type "Float (double-precision)") (TriggeredSeconds :type "Float (double-precision)") (InputAction :type "InputAction Object Reference" :default "/Game/Input/IA_Crouch.IA_Crouch"))
  (:`Started`
    (`self.Crouch`))
  (:`Completed`
    (`self.UnCrouch`)))

(event `EnhancedInput|/Game/Input/IA_Interact`
  (params (ActionValue :type Boolean) (ElapsedSeconds :type "Float (double-precision)") (TriggeredSeconds :type "Float (double-precision)") (InputAction :type "InputAction Object Reference" :default "/Game/Input/IA_Interact.IA_Interact"))
  (bind _camera (`self.Camera`))
  (bind _returnvalue (`SceneComponent.K2_GetComponentLocation` _camera))
  (:`Started`
    (bind _outhit (`KismetSystemLibrary.LineTraceSingle` _returnvalue (+ _returnvalue (* (`SceneComponent.GetForwardVector` _camera) (`self.InteractReach`))) "TraceTypeQuery2"))
    (bind _asbpi_interactable (cast `/Game/Blueprints/BPI_Interactable` (`.HitActor` (`GameplayStatics.BreakHitResult` _outhit))))
    (`/Game/Blueprints/BPI_Interactable.OnInteract` _asbpi_interactable self)))

(event `self.ReceiveBeginPlay`
  (`|ExecutionSequence`
    (:`then_0`
      ;[1 1 1] Initialize our Mapping Context asset as the one this character uses
      (`EnhancedInputSubsystemInterface.AddMappingContext` (pcsubsystem `EnhancedInputLocalPlayerSubsystem` (`GameplayStatics.GetPlayerController` 0)) "/Game/Input/IC_Player.IC_Player" 0 (struct)))
    (:`then_1`
      ;[1 1 1] UI
      (bind _returnvalue (`|CreateWidget` "/Game/UI/W_HUD.W_HUD_C"))
      (`UserWidget.AddToViewport` _returnvalue 0))))

(event `self.ReceiveAnyDamage`
  (params (Damage :type "Float (single-precision)") (DamageType :type "DamageType Object Reference") (InstigatedBy :type "Controller Object Reference") (DamageCauser :type "Actor Object Reference"))
  ;[1 1 1] Tell health component when taken damage, but only if damage isn't from us; uses engine built-in damage system
  (if (!= InstigatedBy (`GameplayStatics.GetPlayerController` 0))
    (`/Game/Blueprints/BP_HealthComponent.Damage` (`self.BP_HealthComponent`) Damage)))

(fn `UserConstructionScript`
  (`|ExecutionSequence`
    (:`then_0`
      (set `CharacterMovementComponent.MaxWalkSpeed` (`self.MoveSpeed`) (`self.CharacterMovement`)))
    (:`then_1`
      (set `CharacterMovementComponent.MaxWalkSpeedCrouched` (* (`self.MoveSpeed`) (`self.CrouchSpeedFactor`)) (`self.CharacterMovement`)))))