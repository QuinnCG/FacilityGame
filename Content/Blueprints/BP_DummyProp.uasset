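; BP_DummyProp is a placeholder interactable prop with a floating text label.
; Each Tick, the label pulses in scale on a sine wave and turns to face the player character's camera.
; OnInteract prints the interaction message, plays a sound at the prop's location and restarts a timeline that animates the mesh scale as feedback.
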(event `self.ReceiveTick`
  (params (DeltaSeconds :type "Float (single-precision)"))
  (`|ExecutionSequence`
    (:`then_0`
      (`SceneComponent.SetRelativeScale3D` (`self.TextRender`) (`KismetMathLibrary.Conv_DoubleToVector` (`KismetMathLibrary.Lerp` 0.9 1.1 (/ (+ (`KismetMathLibrary.Sin` (* (`GameplayStatics.GetTimeSeconds`) 3.0)) 1.0) 2.0)))))
    (:`then_1`
      (`SceneComponent.K2_SetWorldRotation` (`self.TextRender`) (`KismetMathLibrary.Conv_VectorToRotator` (`KismetMathLibrary.Normal` (- (`SceneComponent.K2_GetComponentLocation` (`/Game/Blueprints/BP_PlayerCharacter.Camera` (cast `/Game/Blueprints/BP_PlayerCharacter` (`GameplayStatics.GetPlayerPawn` 0) :!pure true))) (`SceneComponent.K2_GetComponentLocation` (`self.TextRender`))))) false false))))

(event `/Game/Blueprints/BPI_Interactable.OnInteract`
  (params (Player :type "/Game/Blueprints/BP_PlayerCharacter Object Reference"))
  (`KismetSystemLibrary.PrintString` (`self.InteractionMessage`))
  (`GameplayStatics.PlaySoundAtLocation` "/Game/Audio/MetaSounds/MS_DummyPropInteract.MS_DummyPropInteract" (`self.K2_GetActorLocation`) (struct) 1.0 1.0 0.0 null null null null)
  (bind (_direction _scale) (`Timeline|OnInteractedAnim` :!via `PlayFromStart`)
    (:`Update`
      (`SceneComponent.SetRelativeScale3D` (`self.Mesh`) (`KismetMathLibrary.Conv_DoubleToVector` _scale)))))

(fn `UserConstructionScript`)