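; Blueprint function library of raycast helpers that return whether a line trace hit and its hit result.
; Raycast traces on the Visibility channel from an origin along a direction for a given distance, with optional debug drawing.
; RaycastFromView and RaycastFromMouse feed it the first player controller's view point and forward vector, or the mouse cursor's deprojected world position and direction.
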(fn `Raycast`
  (params (Origin :type "Vector Structure") (Direction :type "Vector Structure") (Distance :type "Float (double-precision)") (DisplayType :type "EDrawDebugTrace Enum" :default "None"))
  (returns (DidHit :type Boolean) (HitInfo :type "HitResult Structure"))
  (bind (_outhit _returnvalue) (`KismetSystemLibrary.LineTraceSingle` :`WorldContextObject` (`local.__WorldContext`) :`Start` Origin :`End` (+ Origin (* Direction Distance)) :`TraceChannel` "TraceTypeQuery1" :`DrawDebugType` DisplayType))
  (return _returnvalue _outhit))

(fn `RaycastFromMouse`
  (params (Distance :type "Float (double-precision)") (DisplayType :type "EDrawDebugTrace Enum" :default "None"))
  (returns (DidHit :type Boolean) (OutHit :type "HitResult Structure"))
  (bind (_worldlocation _worlddirection) (`PlayerController.DeprojectMousePositionToWorld` (`GameplayStatics.GetPlayerController` (`local.__WorldContext`))))
  (bind (_didhit _hitinfo) (`self.Raycast` _worldlocation _worlddirection Distance DisplayType (`local.__WorldContext`)))
  (return _didhit _hitinfo))

(fn `RaycastFromView`
  (params (Distance :type "Float (double-precision)") (DisplayType :type "EDrawDebugTrace Enum" :default "None"))
  (returns (DidHit :type Boolean) (HitInfo :type "HitResult Structure"))
  (bind (_location _rotation) (`Controller.GetPlayerViewPoint` (`GameplayStatics.GetPlayerController` (`local.__WorldContext`))))
  (bind (_didhit _hitinfo) (`self.Raycast` _location (`KismetMathLibrary.Conv_RotatorToVector` _rotation) Distance DisplayType (`local.__WorldContext`)))
  (return _didhit _hitinfo))