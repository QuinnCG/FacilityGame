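; Health component that tracks an actor's current health against a maximum.
; Current starts at Max on BeginPlay, and Heal adds to it without exceeding Max.
; Damage lowers Current to no less than zero, then broadcasts OnDamaged with the requested amount.
; OnDeath fires after any Damage call that leaves health at zero, including repeat hits on an already dead owner.
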(event `self.ReceiveBeginPlay`
  (set `self.Current` (`self.Max`)))

(fn `Damage`
  (params (Amount :type "Float (double-precision)"))
  ;[1 1 1] Remove health but prevent it from dipping below 0
  (set `self.Current` (`KismetMathLibrary.FMax` (- (`self.Current`) Amount)))
  (`self.OnDamaged` (`local.Amount`))
  (if (== (`self.Current`) 0.0)
    (`self.OnDeath`)))

(fn `Heal`
  (params (Amount :type "Float (double-precision)"))
  ;[1 1 1] Add health but prevent it from exceeding max
  (set `self.Current` (`KismetMathLibrary.FMin` (+ Amount (`self.Current`)) (`self.Max`))))